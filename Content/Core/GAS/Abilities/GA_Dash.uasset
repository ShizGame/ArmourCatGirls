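; Dash gameplay ability that propels the kitty sandbox character in a direction set by its attached booster armor pieces.
; On commit, it sums the reversed forward vectors of the socketed boosters, so their placement and count shape the dash.
; The resulting movement impulse is multiplied by Strength and a clamped factor inversely proportional to a float attribute on the avatar.
; A short-lived debug arrow shows the impulse before the ability ends.
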(event Ability|EventActivateAbility
  (bind _returnvalue (Ability|CommitAbility))
  (if _returnvalue
    (bind _ascbp_sandbox_character_kitty (Utilities|Casting|CastToCBP_SandboxCharacter_Kitty (Ability|GetAvatarActorfromActorInfo))
      (:then
        (Variables|Default|SetCharacterKitty _ascbp_sandbox_character_kitty)
        (bind _values (Utilities|Map|Values (Variables|/Game/Blueprints/RetargetedCharacters/CBP_SandboxCharacter_Kitty.CBP_SandboxCharacter_Kitty_C|GetActorOnSockets _ascbp_sandbox_character_kitty)))
        (for _array_element _values
          (bind _asa_armor_booster (Utilities|Casting|CastToA_Armor_Booster _array_element))
          (Variables|Default|SetFinalVector (+ (Variables|Default|GetFinalVector) (* (Transformation|GetActorForwardVector _asa_armor_booster) -1))))
        (Physics|AddImpulse (Variables|/Script/Engine.Character|GetCharacterMovement (Variables|Default|GetCharacterKitty)) (* (Variables|Default|GetFinalVector) (Math|Float|Clamp(Float) (/ 5e+01 (.ReturnValue (Ability|Attribute|GetFloatAttribute (Ability|GetAvatarActorfromActorInfo) "(AttributeName=\"Weight\",Attribute=/Script/ArmourCatGirls.AttributeSetCATGirl:Weight,AttributeOwner=\"/Script/CoreUObject.Class'/Script/ArmourCatGirls.AttributeSetCATGirl'\")"))) 0.1 2.0) (Variables|Default|GetStrength)) false)
        (Rendering|Debug|DrawDebugArrow (Transformation|GetActorLocation (Variables|Default|GetCharacterKitty)) (+ (Transformation|GetActorLocation (Variables|Default|GetCharacterKitty)) (/ (* (Variables|Default|GetFinalVector) (Math|Float|Clamp(Float) (/ 5e+01 (.ReturnValue (Ability|Attribute|GetFloatAttribute (Ability|GetAvatarActorfromActorInfo) "(AttributeName=\"Weight\",Attribute=/Script/ArmourCatGirls.AttributeSetCATGirl:Weight,AttributeOwner=\"/Script/CoreUObject.Class'/Script/ArmourCatGirls.AttributeSetCATGirl'\")"))) 0.1 2.0) (Variables|Default|GetStrength)) 1000)) 25.0 "(R=1.000000,G=0.000000,B=0.047706,A=1.000000)" 1.0 5.0)
        (Ability|EndAbility))
      (:CastFailed
        (Ability|EndAbility)))
    (else
      (Ability|EndAbility))))