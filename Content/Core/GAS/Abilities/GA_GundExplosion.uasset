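; GA_GundExplosion is a Gameplay Ability that sets off an explosion around its avatar, damaging nearby actors.
; On activation it executes the explosion GameplayCue, then runs a sphere overlap at the avatar's location, ignoring the avatar.
; Each overlapped actor with an Ability System Component applies GE_SimpleDamage to itself, with no team or line-of-sight check, and the ability then ends.
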(event Ability|EventActivateAbility
  (bind _returnvalue (Ability|GetAvatarActorfromActorInfo))
  (Utilities|FlowControl|Sequence
    (:then_0
      (GameplayCue|ExecuteGameplayCue :GameplayCueTag "(TagName=\"GameplayCue.Explosion\")"))
    (:then_1
      (bind _outactors (Collision|SphereOverlapActors (Transformation|GetActorLocation _returnvalue) (Variables|Default|GetSphere%20Radius) (Utilities|Array|MakeArray "ObjectTypeQuery1" "ObjectTypeQuery2" "ObjectTypeQuery3") 0 (Utilities|Array|MakeArray _returnvalue)))
      (for _array_element _outactors
        (Utilities|IsValid (Ability|GetAbilitySystemComponent _array_element)
          (:Is%20Valid
            (GameplayEffects|ApplyGameplayEffectToSelf :self (Ability|GetAbilitySystemComponent _array_element) :GameplayEffectClass "/Game/Core/GAS/Effects/GE_SimpleDamage.GE_SimpleDamage_C"))))
      (Ability|EndAbility))))