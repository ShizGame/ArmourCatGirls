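; GA_Shoot is a Gameplay Ability for automatic fire, shooting on activation and on a looping timer until input release ends it.
; After committing, it derives the firing interval from an avatar float attribute.
; Each shot gets muzzle location and aim through avatar messages, then spawns BP_Bullet with random spread, attribute-driven speed and the bullet tag container.
; The Bullet.Multiplay tag turns each shot into three side-by-side bullets.
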(event Custom|Shooting
  (bind _returnvalue (Math|Random|RandomFloatinRange -3.0 3.0))
  (bind _returnvalue_2 (Ability|GetAvatarActorfromActorInfo))
  (bind _bullettagcontainer (Variables|Default|GetBulletTagContainer))
  (bind _returnvalue_3 (Ability|Attribute|GetFloatAttribute _returnvalue_2 "(AttributeName=\"StartBulletsSpeed\",Attribute=/Script/ArmourCatGirls.AttributeSetWeapon:StartBulletsSpeed,AttributeOwner=\"/Script/CoreUObject.Class'/Script/ArmourCatGirls.AttributeSetWeapon'\")"))
  (bind (_location _relevant) (Class|BPIGun|GetMuzzleLocation(Message) (Ability|GetAvatarActorfromActorInfo)))
  (if _relevant
    (bind _rotation (Class|BPIGun|GetShoottingRotation(Message) (Ability|GetAvatarActorfromActorInfo)))
    (if (GameplayTags|HasTag (Variables|Default|GetBulletTagContainer) "(TagName=\"Bullet.Multiplay\")")
      (for _index (range -1 1)
        (Game|SpawnActorfromClass "/Game/Core/Blueprints/Actors/BP_Bullet.BP_Bullet_C" (Math|Transform|MakeTransform (+ _location (* (Math|Vector|GetRightVector (Math|Rotator|MakeRotator (+ (.Roll (Math|Rotator|BreakRotator _rotation)) _returnvalue) (+ (.Pitch (Math|Rotator|BreakRotator _rotation)) _returnvalue) (+ (.Yaw (Math|Rotator|BreakRotator _rotation)) _returnvalue))) _index 1e+01)) (Math|Rotator|MakeRotator (+ (.Roll (Math|Rotator|BreakRotator _rotation)) _returnvalue) (+ (.Pitch (Math|Rotator|BreakRotator _rotation)) _returnvalue) (+ (.Yaw (Math|Rotator|BreakRotator _rotation)) _returnvalue)) "1.000000,1.000000,1.000000") "Undefined" "MultiplyWithRoot" 0 _returnvalue_3 _bullettagcontainer 0))
      (else
        (Game|SpawnActorfromClass "/Game/Core/Blueprints/Actors/BP_Bullet.BP_Bullet_C" (Math|Transform|MakeTransform _location (Math|Rotator|MakeRotator (+ (.Roll (Math|Rotator|BreakRotator _rotation)) _returnvalue) (+ (.Pitch (Math|Rotator|BreakRotator _rotation)) _returnvalue) (+ (.Yaw (Math|Rotator|BreakRotator _rotation)) _returnvalue)) "1.000000,1.000000,1.000000") "Undefined" "MultiplyWithRoot" 0 _returnvalue_3 _bullettagcontainer 0)))
    (else
      (Ability|EndAbility))))

(event Ability|EventActivateAbility
  (bind _returnvalue (Ability|GetAvatarActorfromActorInfo))
  (bind (_bsuccessfullyfoundattribute _returnvalue_2) (Ability|Attribute|GetFloatAttribute _returnvalue "(AttributeName=\"FireRate\",Attribute=/Script/ArmourCatGirls.AttributeSetWeapon:FireRate,AttributeOwner=\"/Script/CoreUObject.Class'/Script/ArmourCatGirls.AttributeSetWeapon'\")"))
  (bind _returnvalue_3 (Ability|CommitAbility))
  (if _returnvalue_3
    (if _bsuccessfullyfoundattribute
      (Utilities|Time|SetTimerbyEvent (delegate Custom|Shooting) (/ 1.0 _returnvalue_2) true)
      (CallFunction|Shooting)
      (Ability|Tasks|WaitInputRelease false
        (:OnRelease
          (Ability|EndAbility)))
      (else
        (Ability|EndAbility)))
    (else
      (Ability|EndAbility))))