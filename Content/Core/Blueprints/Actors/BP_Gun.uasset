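; BP_Gun is a gun actor that fires through the Gameplay Ability System and is customized with modules.
; On BeginPlay it adds its input mapping and grants GA_Shoot, which the fire action presses and releases by input ID.
; Adding or removing a module removes previously applied effects, then rebuilds the ability's bullet tags and reapplies gameplay effects from GunModulesArchive.
; Helper functions expose the muzzle socket location and the actor's rotation for shooting.
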(event Custom|AddGunModule
  (params (NewGunModule :type E_GunModules%20Enum :default "NewEnumerator3"))
  (Utilities|Array|Add (Variables|Default|GetGunModules) NewGunModule)
  (CallFunction|ApplyGunModules))

(event Custom|RemoveGunModule
  (params (GunModule :type E_GunModules%20Enum :default "NewEnumerator3"))
  (Utilities|Array|RemoveItem (Variables|Default|GetGunModules) GunModule)
  (CallFunction|ApplyGunModules))

(event Custom|ApplyGunModules
  (Utilities|FlowControl|Sequence
    (:then_0
      (Variables|/Game/Core/GAS/Abilities/GA_Shoot.GA_Shoot_C|SetBulletTagContainer (Variables|Default|GetGAShoot) "")
      (for _array_element (Variables|Default|GetEffectsFromModules)
        (GameplayEffects|RemoveActiveGameplayEffect (Variables|Default|GetAbilitySystem) _array_element -1)))
    (:then_1
      (for _array_element_2 (Variables|Default|GetGunModules)
        (GameplayTags|AppendGameplayTagContainers (Variables|/Game/Core/GAS/Abilities/GA_Shoot.GA_Shoot_C|GetBulletTagContainer (Variables|Default|GetGAShoot)) (.BulletTags (Utilities|Struct|BreakS_GunModule (.Value (Utilities|Map|Find (Variables|/Game/Core/GunModules/PDA_GunModule.PDA_GunModule_C|GetGunModules (Variables|Default|GetGunModulesArchive)) _array_element_2)))))
        (for _array_element_3 (.GunEffects (Utilities|Struct|BreakS_GunModule (.Value (Utilities|Map|Find (Variables|/Game/Core/GunModules/PDA_GunModule.PDA_GunModule_C|GetGunModules (Variables|Default|GetGunModulesArchive)) _array_element_2))))
          (bind _returnvalue (GameplayEffects|ApplyGameplayEffectToSelf :self (Variables|Default|GetAbilitySystem) :GameplayEffectClass _array_element_3))
          (Utilities|Array|Add (Variables|Default|GetEffectsFromModules) _returnvalue))))))

(event Input|EnhancedActionEvents|EnhancedInputActionIA_Fire
  (params (ActionValue :type Boolean) (ElapsedSeconds :type Float%20%28double-precision%29) (TriggeredSeconds :type Float%20%28double-precision%29) (InputAction :type Input%20Action%20Object%20Reference :default "/Game/Core/Input/IA_Fire.IA_Fire"))
  (bind _abilitysystem (Variables|Default|GetAbilitySystem))
  (:Triggered
    (Class|AbilitySystemComponent|PressInputID _abilitysystem))
  (:Canceled
    (Class|AbilitySystemComponent|ReleaseInputID _abilitysystem :!label _label))
  (:Completed
    (goto _label)))

(event EventBeginPlay
  (bind _abilitysystem (Variables|Default|GetAbilitySystem))
  (Input|AddMappingContext (PlayerController|LocalPlayerSubsystems|GetEnhancedInputLocalPlayerSubsystem (Game|GetPlayerController 0)) "/Game/Core/Input/IMC_Guns.IMC_Guns" 0 "(bIgnoreAllPressedKeysUntilRelease=True,bForceImmediately=False,bNotifyUserSettings=False)")
  (bind _returnvalue (GameplayAbilities|GiveAbility _abilitysystem "/Game/Core/GAS/Abilities/GA_Shoot.GA_Shoot_C" 0 0))
  (Variables|Default|SetGAShoot (.AsGA%20Shoot (Utilities|Casting|CastToGA_Shoot (.ReturnValue (Ability|GameplayAbility|GetGameplayAbilityfromSpecHandle _abilitysystem _returnvalue))))))

(fn ConstructionScript)

(fn GetMuzzleLocation
  (bind _staticmesh (Variables|Default|GetStaticMesh))
  (bind _returnvalue (Transformation|GetSocketLocation _staticmesh "Muzzle"))
  (return _returnvalue (Utilities|Operators|NotEqual(!=) :A _returnvalue :ErrorTolerance 1.0)))

(fn GetShoottingRotation
  (return (Transformation|GetActorRotation)))