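; BP_Bullet is a projectile that damages what it overlaps, ignoring other bullets, with initial speed set in the construction script.
; On overlap it applies GE_SimpleDamage through the target's Ability System Component.
; Gameplay tags vary the behavior: Explosive adds radial damage to other WorldDynamic and WorldStatic actors and draws a debug sphere.
; The bullet destroys itself after a hit unless tagged Piercing.
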(event OnComponentBeginOverlap(Sphere)
  (params (OverlappedComponent :type Primitive%20Component%20Object%20Reference) (OtherActor :type Actor%20Object%20Reference) (OtherComp :type Primitive%20Component%20Object%20Reference) (OtherBodyIndex :type Integer) (bFromSweep :type Boolean) (SweepResult :type Hit%20Result%20Structure%20%28by%20ref%29))
  (bind _returnvalue (Ability|GetAbilitySystemComponent OtherActor))
  (bind _returnvalue_2 (Transformation|GetActorLocation))
  (bind _explosionradius (Variables|Default|GetExplosionRadius))
  (Utilities|Casting|CastToBP_Bullet OtherActor
    (:CastFailed
      (Utilities|FlowControl|Sequence
        (:then_0
          (Utilities|IsValid _returnvalue
            (:Is%20Valid
              (GameplayEffects|ApplyGameplayEffectToSelf :self _returnvalue :GameplayEffectClass "/Game/Core/GAS/Effects/GE_SimpleDamage.GE_SimpleDamage_C"))))
        (:then_1
          (if (GameplayTags|HasTag (Variables|Default|GetTagContainer) "(TagName=\"Bullet.Explosive\")")
            (bind _outactors (Collision|SphereOverlapActors _returnvalue_2 _explosionradius (Utilities|Array|MakeArray "ObjectTypeQuery2" "ObjectTypeQuery1") 0 (Utilities|Array|MakeArray OtherActor)))
            (Rendering|Debug|DrawDebugSphere _returnvalue_2 _explosionradius 12 "(R=1.000000,G=0.000000,B=0.000000,A=1.000000)" 0.0 0.3)
            (for _array_element _outactors
              (Utilities|IsValid (Ability|GetAbilitySystemComponent _array_element)
                (:Is%20Valid
                  (GameplayEffects|ApplyGameplayEffectToSelf :self (Ability|GetAbilitySystemComponent _array_element) :GameplayEffectClass "/Game/Core/GAS/Effects/GE_SimpleDamage.GE_SimpleDamage_C"))))))
        (:then_4
          (if (not (GameplayTags|HasTag (Variables|Default|GetTagContainer) "(TagName=\"Bullet.Piercing\")"))
            (Actor|DestroyActor)))))))

(fn ConstructionScript
  (Variables|/Script/Engine.ProjectileMovementComponent|SetInitialSpeed (Variables|Default|GetProjectileMovement) (Variables|Default|GetInitial%20Speed)))