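; BP_DestructibleWall is a wall actor that flashes when hit and is destroyed when its attribute runs out.
; On BeginPlay it listens for attribute changes on its Ability System component, flashing on every change and destroying itself when the new value reaches zero or below.
; The flash writes the current game time into custom primitive data on the static mesh, presumably leaving the material to animate it.
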(event Custom|HitEmissive
  (CallFunction|InitFlash))

(event Custom|InitFlash
  (Rendering|Material|SetCustomPrimitiveDataFloat (Variables|Default|GetStaticMesh) 0 (Utilities|Time|GetTimeSeconds)))

(event EventBeginPlay
  (bind _newvalue (|ListenforAttributeChange (Variables|Default|GetAbilitySystem) "(AttributeName=\"Health\",Attribute=/Script/ArmourCatGirls.AttributeSetMain:Health,AttributeOwner=\"/Script/CoreUObject.Class'/Script/ArmourCatGirls.AttributeSetMain'\")")
    (:OnAttributeChanged
      (CallFunction|HitEmissive)
      (if (<= _newvalue 0.0)
        (Actor|DestroyActor)))))

(fn ConstructionScript)