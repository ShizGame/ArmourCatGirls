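; BP_BaseArmore is a base armour actor whose appearance is chosen by its socket name.
; The construction script looks up SocketName in the DTSocketsMeshVariants data table and, if the row exists, applies its armour mesh and world scale to the StaticMesh component.
; The event graph holds only disabled placeholder events, so the Blueprint adds no runtime logic.
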(event EventBeginPlay)

(event Collision|EventActorBeginOverlap
  (params (OtherActor :type Actor%20Object%20Reference)))

(event EventTick
  (params (DeltaSeconds :type Float%20%28single-precision%29)))

(fn ConstructionScript
  (bind _returnvalue (Class|DataTableFunctionLibrary|DoesDataTableRowExist (Variables|Default|GetDTSocketsMeshVariants) (Variables|Default|GetSocketName)))
  (if _returnvalue
    (bind _returnvalue_2 (Utilities|GetDataTableRow (Variables|Default|GetDTSocketsMeshVariants) (Variables|Default|GetSocketName))
      (:then
        (Components|StaticMesh|SetStaticMesh (Variables|Default|GetStaticMesh) (.ArmourMesh (Utilities|Struct|BreakSSocketModule _returnvalue_2)))
        (Transformation|SetWorldScale3D (Variables|Default|GetStaticMesh) (.Scale (Utilities|Struct|BreakSSocketModule _returnvalue_2)))))))